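; Player 1 pawn for the Cage Versus mode, handling its input setup and height-based collision scoring.
; On BeginPlay it adds the Player 1 Enhanced Input mapping context and caches the game mode.
; When its Playerbase component hits player pawn 0, it compares the Z positions of pawns 0 and 1.
; The game mode awards P1 points if pawn 0 is higher, P2 if lower, none if level.
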(event `self.ReceiveBeginPlay`
  ; Add Mapping
  (bind _asplayer_controller (cast `PlayerController` (`self.GetController`)))
  (bind _returnvalue (pcsubsystem `EnhancedInputLocalPlayerSubsystem` _asplayer_controller))
  (`/Engine/EditorBlueprintResources/StandardMacros.IsValid` _returnvalue
    (:`Is Valid`
      (`EnhancedInputSubsystemInterface.AddMappingContext` _returnvalue "/Game/Actions/IM_Player1.IM_Player1" 0 (struct))
      (bind _asbp_gamemode_cage_versus (cast `/Game/BP_Gamemode_CageVersus` (`GameplayStatics.GetGameMode`)))
      (set `self.As BP Gamemode Cage Versus` _asbp_gamemode_cage_versus))))

(event `self.Playerbase.OnComponentHit`
  (params (HitComponent :type "PrimitiveComponent Object Reference") (OtherActor :type "Actor Object Reference") (OtherComp :type "PrimitiveComponent Object Reference") (NormalImpulse :type "Vector Structure") (Hit :type "HitResult Structure (by ref)"))
  (bind _returnvalue (`GameplayStatics.GetPlayerPawn` 0))
  (bind (_returnvalue_x _returnvalue_y _returnvalue_z) (`KismetMathLibrary.BreakVector` (`self.K2_GetActorLocation` (`GameplayStatics.GetPlayerPawn` 1))))
  (bind (_returnvalue_x_2 _returnvalue_y_2 _returnvalue_z_2) (`KismetMathLibrary.BreakVector` (`self.K2_GetActorLocation` _returnvalue)))
  ; Punteggio Player
  (if (== OtherActor _returnvalue)
    (`/Engine/EditorBlueprintResources/StandardMacros.CompareFloat` _returnvalue_z_2 _returnvalue_z
      (:`>`
        (if true
          (bind _asbp_gamemode_cage_versus (cast `/Game/BP_Gamemode_CageVersus` (`GameplayStatics.GetGameMode`)))
          (bind _output_get (set `self.GamemodeRef` _asbp_gamemode_cage_versus))
          (`/Game/BP_Gamemode_CageVersus.P1AddPoints` _output_get)))
      (:`<`
        (if true
          (bind _asbp_gamemode_cage_versus_2 (cast `/Game/BP_Gamemode_CageVersus` (`GameplayStatics.GetGameMode`)))
          (bind _output_get_2 (set `self.GamemodeRef` _asbp_gamemode_cage_versus_2))
          (`/Game/BP_Gamemode_CageVersus.P2AddPoints` _output_get_2))))))

(fn `UserConstructionScript`)