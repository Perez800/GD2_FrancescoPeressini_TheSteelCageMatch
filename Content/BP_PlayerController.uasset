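; Player controller for two local players, routing separate rotate and jump input actions to pawns 0 and 1 by player index.
; Rotation adds yaw input, while jumping applies a physics impulse to the pawn's static mesh along its arrow component's forward vector.
; Jumps require that player's grounded flag, which is written through SetGrounded.
; The pause action opens the GamePause widget, shows player 0's cursor, switches to UI-only input and pauses the game.
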(event `EnhancedInput|/Game/Actions/IA_Rotate`
  (params (ActionValue :type "Float (double-precision)") (ElapsedSeconds :type "Float (double-precision)") (TriggeredSeconds :type "Float (double-precision)") (InputAction :type "InputAction Object Reference" :default "/Game/Actions/IA_Rotate.IA_Rotate"))
  ; Comandi Giocatori
  (:`Triggered`
    (`Pawn.AddControllerYawInput` (`GameplayStatics.GetPlayerPawn` 0) ActionValue)))

(event `EnhancedInput|/Game/Actions/IA_Jump`
  (params (ActionValue :type Boolean) (ElapsedSeconds :type "Float (double-precision)") (TriggeredSeconds :type "Float (double-precision)") (InputAction :type "InputAction Object Reference" :default "/Game/Actions/IA_Jump.IA_Jump"))
  (bind _returnvalue (`GameplayStatics.GetPlayerPawn` 0))
  ; Comandi Giocatori
  (:`Started`
    (if (`self.IsGrounded0`)
      (`PrimitiveComponent.AddImpulse` (`self.GetComponentByClass` _returnvalue "/Script/Engine.StaticMeshComponent") (* (`SceneComponent.GetForwardVector` (`self.GetComponentByClass` _returnvalue "/Script/Engine.ArrowComponent")) 130000) "None" false))))

(event `EnhancedInput|/Game/Actions/IA_RotateAlt`
  (params (ActionValue :type "Float (double-precision)") (ElapsedSeconds :type "Float (double-precision)") (TriggeredSeconds :type "Float (double-precision)") (InputAction :type "InputAction Object Reference" :default "/Game/Actions/IA_RotateAlt.IA_RotateAlt"))
  ; Comandi Giocatori
  (:`Triggered`
    (`Pawn.AddControllerYawInput` (`GameplayStatics.GetPlayerPawn` 1) ActionValue)))

(event `EnhancedInput|/Game/Actions/IA_JumpAlt`
  (params (ActionValue :type Boolean) (ElapsedSeconds :type "Float (double-precision)") (TriggeredSeconds :type "Float (double-precision)") (InputAction :type "InputAction Object Reference" :default "/Game/Actions/IA_JumpAlt.IA_JumpAlt"))
  (bind _returnvalue (`GameplayStatics.GetPlayerPawn` 1))
  ; Comandi Giocatori
  (:`Started`
    (if (`self.IsGrounded1`)
      (`PrimitiveComponent.AddImpulse` (`self.GetComponentByClass` _returnvalue "/Script/Engine.StaticMeshComponent") (* (`SceneComponent.GetForwardVector` (`self.GetComponentByClass` _returnvalue "/Script/Engine.ArrowComponent")) 130000) "None" false))))

(event `EnhancedInput|/Game/Actions/IA_Pause`
  (params (ActionValue :type Boolean) (ElapsedSeconds :type "Float (double-precision)") (TriggeredSeconds :type "Float (double-precision)") (InputAction :type "InputAction Object Reference" :default "/Game/Actions/IA_Pause.IA_Pause"))
  (bind _returnvalue (`GameplayStatics.GetPlayerController` 0))
  ; Comandi Giocatori
  (:`Started`
    (bind _returnvalue_2 (`|CreateWidget` "/Game/UI/GamePause.GamePause_C"))
    (`UserWidget.AddToViewport` _returnvalue_2 0)
    (set `PlayerController.bShowMouseCursor` true _returnvalue)
    (`WidgetBlueprintLibrary.SetInputMode_UIOnlyEx` _returnvalue null)
    (`GameplayStatics.SetGamePaused` true)))

(fn `SetGrounded`
  (params (Index :type Integer) (Value :type Boolean))
  (switch `int` Index
    (:`0`
      (set `self.IsGrounded0` Value))
    (:`1`
      (set `self.IsGrounded1` Value))))

(fn `UserConstructionScript`)